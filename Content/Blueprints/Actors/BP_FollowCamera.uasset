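; Camera actor that smoothly follows a FollowTarget actor, shifted along the direction the target faces.
; Each Tick, UpdateCameraPosition uses VInterpTo to move the actor toward the target point at InterpSpeed.
; SetFollowTarget supplies the target's location, keeping the camera's own height when ShouldLockHeight is set.
; SetCameraOffset scales the target's forward vector by CameraOffset, applying only X and Z, so Y follows without offset.
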(event `self.ReceiveTick`
  (params (DeltaSeconds :type "Float (single-precision)"))
  (`self.UpdateCameraPosition`))

(fn `SetCameraOffset`
  (returns (X :type "Float (double-precision)") (Z :type "Float (double-precision)"))
  (bind (_returnvalue_x _returnvalue_y _returnvalue_z) (`KismetMathLibrary.BreakVector` (* (`self.GetActorForwardVector` (`self.FollowTarget`)) (`self.CameraOffset`))))
  (return _returnvalue_x _returnvalue_z))

(fn `SetFollowTarget`
  (returns (X :type "Float (double-precision)") (Y :type "Float (double-precision)") (Z :type "Float (double-precision)"))
  (bind (_returnvalue_x _returnvalue_y _returnvalue_z) (`KismetMathLibrary.BreakVector` (`self.K2_GetActorLocation`)))
  (bind (_returnvalue_x_2 _returnvalue_y_2 _returnvalue_z_2) (`KismetMathLibrary.BreakVector` (`self.K2_GetActorLocation` (`self.FollowTarget`))))
  (return _returnvalue_x_2 _returnvalue_y_2 (select `bool` (`self.bShouldLockHeight`) :`false` _returnvalue_z_2 :`true` _returnvalue_z)))

(fn `UpdateCameraPosition`
  (bind (_x _z) (`self.SetCameraOffset`))
  (bind (_x_2 _y _z_2) (`self.SetFollowTarget`))
  (`self.K2_SetActorLocation` (`KismetMathLibrary.VInterpTo` (`self.K2_GetActorLocation`) (+ (`KismetMathLibrary.MakeVector` _x_2 _y _z_2) (`KismetMathLibrary.MakeVector` _x 0.0 _z)) (`GameplayStatics.GetWorldDeltaSeconds`) (`self.Interp Speed`))))

(fn `UserConstructionScript`)